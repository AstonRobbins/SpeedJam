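; BP_Checkpoint is a single-use checkpoint that saves a respawn location when the third-person character enters its box.
; A looping timer periodically pulses a height-adjusted Niagara marker while ShowNiagara is set.
; On overlap it disables the marker, writes the RespPosition location to LastCheckpoint on BP_ThirdPersonGameMode, spawns an airflow effect, then destroys itself after a short delay.
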(event OnComponentBeginOverlap(Box)
  (params (OverlappedComponent :type Primitive%20Component%20Object%20Reference) (OtherActor :type Actor%20Object%20Reference) (OtherComp :type Primitive%20Component%20Object%20Reference) (OtherBodyIndex :type Integer) (bFromSweep :type Boolean) (SweepResult :type Hit%20Result%20Structure%20%28by%20ref%29))
  (bind _resp_position (Variables|Default|Getresp_Position))
  (bind _returnvalue (Transformation|GetWorldLocation _resp_position))
  (bind (_x _y _z) (Math|Vector|BreakVector _returnvalue))
  (Utilities|Casting|CastToBP_ThirdPersonCharacter OtherActor)
  (Variables|Default|SetShowNiagara false)
  (bind _asbp_third_person_game_mode (Utilities|Casting|CastToBP_ThirdPersonGameMode (Game|GetGameMode)))
  (Variables|/Game/ThirdPerson/Blueprints/BP_ThirdPersonGameMode.BP_ThirdPersonGameMode_C|SetLastCheckpoint _asbp_third_person_game_mode _returnvalue)
  (Niagara|SpawnSystematLocation "/Game/Air_Magic/VFX_Niagara/NS_Air_Magic_Airflow.NS_Air_Magic_Airflow" (Math|Vector|MakeVector _x _y (+ _z (Variables|Default|GetNiagaraHeight))))
  (Components|Activation|Deactivate (Variables|Default|GetNiagara))
  (Utilities|FlowControl|Delay 2.0)
  (Utilities|IsValid 0
    (:Is%20Valid
      (Actor|DestroyActor))))

(event Custom|ShowCheckpoint
  (if (Variables|Default|GetShowNiagara)
    (Components|Activation|Activate (Variables|Default|GetNiagara) false)
    (Utilities|FlowControl|Delay 3.0)
    (Components|Activation|Deactivate (Variables|Default|GetNiagara))))

(event EventBeginPlay
  (Transformation|SetRelativeLocation (Variables|Default|GetNiagara) (Math|Vector|MakeVector 0.0 0.0 (Variables|Default|GetNiagaraHeight)) false false)
  (Utilities|Time|SetTimerbyEvent (delegate Custom|ShowCheckpoint) 1.0 true))

(event Collision|EventActorBeginOverlap
  (params (OtherActor :type Actor%20Object%20Reference)))

(event EventTick
  (params (DeltaSeconds :type Float%20%28single-precision%29)))

(fn ConstructionScript)