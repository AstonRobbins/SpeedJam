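; BP_ManaBall is a mana pickup that restores the mana of the third-person player character.
; On actor overlap it casts to BP_ThirdPersonCharacter and adds a fixed amount of Mana, topping up to the hardcoded maximum when nearly full.
; The ball destroys itself only after granting mana, so it stays in the world when the character is already full.
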(event EventBeginPlay)

(event Collision|EventActorBeginOverlap
  (params (OtherActor :type Actor%20Object%20Reference))
  (bind _asbp_third_person_character (Utilities|Casting|CastToBP_ThirdPersonCharacter OtherActor))
  (if (< (Variables|/Game/ThirdPerson/Blueprints/BP_ThirdPersonCharacter.BP_ThirdPersonCharacter_C|GetMana _asbp_third_person_character) 80)
    (Variables|/Game/ThirdPerson/Blueprints/BP_ThirdPersonCharacter.BP_ThirdPersonCharacter_C|SetMana _asbp_third_person_character (+ (Variables|/Game/ThirdPerson/Blueprints/BP_ThirdPersonCharacter.BP_ThirdPersonCharacter_C|GetMana _asbp_third_person_character) 20))
    (Actor|DestroyActor :!label _label)
    (elif (< (Variables|/Game/ThirdPerson/Blueprints/BP_ThirdPersonCharacter.BP_ThirdPersonCharacter_C|GetMana _asbp_third_person_character) 100)
      (Variables|/Game/ThirdPerson/Blueprints/BP_ThirdPersonCharacter.BP_ThirdPersonCharacter_C|SetMana _asbp_third_person_character (+ (Variables|/Game/ThirdPerson/Blueprints/BP_ThirdPersonCharacter.BP_ThirdPersonCharacter_C|GetMana _asbp_third_person_character) (- 100 (Variables|/Game/ThirdPerson/Blueprints/BP_ThirdPersonCharacter.BP_ThirdPersonCharacter_C|GetMana _asbp_third_person_character))))
      (goto _label))))

(event EventTick
  (params (DeltaSeconds :type Float%20%28single-precision%29)))

(fn ConstructionScript)