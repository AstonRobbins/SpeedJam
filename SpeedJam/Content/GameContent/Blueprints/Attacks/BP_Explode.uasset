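; Explosion actor that applies a one-shot radial blast on spawn.
; BeginPlay runs a multi sphere trace on the Visibility channel around its Sphere and pushes each hit actor away from the center.
; Player characters are launched and lose health, Enemy-tagged actors have skeletal mesh physics enabled before the force, and physics-simulating static meshes receive force.
; A Delay inside the hit loop then destroys the actor, so cleanup depends on getting hits.
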(event Collision|EventActorBeginOverlap
  (params (OtherActor :type Actor%20Object%20Reference)))

(event EventBeginPlay
  (bind _sphere (Variables|Default|GetSphere))
  (bind _returnvalue (Transformation|GetWorldLocation _sphere))
  (bind (_outhits _returnvalue_2) (Collision|MultiSphereTraceByChannel _returnvalue _returnvalue 5e+02 "TraceTypeQuery1" false 0 "None"))
  (for _array_element _outhits
    (Variables|Default|SetArray%20Element _array_element)
    (if _returnvalue_2
      (bind _asbp_third_person_character (Utilities|Casting|CastToBP_ThirdPersonCharacter (.hitactor (Variables|Default|GetArray%20Element)))
        (:then
          (Character|LaunchCharacter _asbp_third_person_character (* (- (Transformation|GetActorLocation _asbp_third_person_character) (Transformation|GetWorldLocation (Variables|Default|GetSphere))) 2e+01) false false)
          (Variables|/Game/ThirdPerson/Blueprints/BP_ThirdPersonCharacter.BP_ThirdPersonCharacter_C|SetHealth _asbp_third_person_character (- (Variables|/Game/ThirdPerson/Blueprints/BP_ThirdPersonCharacter.BP_ThirdPersonCharacter_C|GetHealth _asbp_third_person_character) 5e+01)))
        (:CastFailed
          (if (Actor|ActorHasTag (.hitactor (Variables|Default|GetArray%20Element)) "Enemy")
            (Physics|SetSimulatePhysics (Actor|GetComponentbyClass (.hitactor (Variables|Default|GetArray%20Element)) "/Script/Engine.SkeletalMeshComponent") true)
            (Physics|AddForce (Actor|GetComponentbyClass (.hitactor (Variables|Default|GetArray%20Element)) "/Script/Engine.SkeletalMeshComponent") (* (- (Transformation|GetActorLocation (.hitactor (Variables|Default|GetArray%20Element))) (Transformation|GetWorldLocation (Variables|Default|GetSphere))) 1e+04) "None" false)
            (else
              (Utilities|IsValid (Actor|GetComponentbyClass (.hitactor (Variables|Default|GetArray%20Element)) "/Script/Engine.StaticMeshComponent")
                (:Is%20Valid
                  (if (Physics|IsSimulatingPhysics (Actor|GetComponentbyClass (.hitactor (Variables|Default|GetArray%20Element)) "/Script/Engine.StaticMeshComponent") "None")
                    (Physics|AddForce (Actor|GetComponentbyClass (.hitactor (Variables|Default|GetArray%20Element)) "/Script/Engine.StaticMeshComponent") (* (- (Transformation|GetActorLocation (.hitactor (Variables|Default|GetArray%20Element))) (Transformation|GetWorldLocation (Variables|Default|GetSphere))) 1e+04) "None" false)))
                (:Is%20Not%20Valid
                  _)))))))
    (Utilities|FlowControl|Delay 2.0)
    (Utilities|IsValid self
      (:Is%20Valid
        (Actor|DestroyActor)))))

(fn ConstructionScript)