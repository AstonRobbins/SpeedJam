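; Enemy AI controller that runs the Enemy_BT behavior tree for a BP_Enemy pawn.
; On BeginPlay it caches the pawn, stores the player character as CurrentTarget and writes CurrentState to the AIState blackboard key.
; A looping timer fires AIAttack, which repeatedly sets that state to a fixed enum value.
; A separate Pawn_Attack event forwards attack requests to the pawn's Attack function.
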(event Custom|Pawn_Attack
  (Default|Attack (Variables|Default|GetEnemyPawn)))

(event Custom|AIAttack
  (Variables|Default|SetCurrentState "NewEnumerator1")
  (AI|Components|Blackboard|SetValueasEnum (AI|GetBlackboard 0) (Utilities|Name|MakeLiteralName "AIState") (Variables|Default|GetCurrentState)))

(event EventBeginPlay
  (bind _asbp_enemy (Utilities|Casting|CastToBP_Enemy (Pawn|GetControlledPawn)))
  (Variables|Default|SetEnemyPawn _asbp_enemy)
  (AI|RunBehaviorTree "/Game/GameContent/Blueprints/Enemies/Enemy_BT.Enemy_BT")
  (Variables|Default|SetCurrentTarget (Game|GetPlayerCharacter 0))
  (AI|Components|Blackboard|SetValueasEnum (AI|GetBlackboard 0) (Utilities|Name|MakeLiteralName "AIState") (Variables|Default|GetCurrentState))
  (Utilities|Time|SetTimerbyEvent (delegate Custom|AIAttack) 2.0 true))

(event EventTick
  (params (DeltaSeconds :type Float%20%28single-precision%29)))

(fn ConstructionScript)